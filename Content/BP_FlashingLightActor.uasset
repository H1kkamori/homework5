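; Actor that flashes its point light a set number of times when play begins.
; BeginPlay enters a DoN gate capped by NumFlashes, which toggles the light's visibility twice with a FlashInterval delay after each toggle, then loops back into the gate.
; Each pass returns the light to its starting visibility.
; The construction script is empty, and NewFunction_0 holds only an empty loop.
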(event `self.ReceiveBeginPlay`
  (`/Engine/EditorBlueprintResources/StandardMacros.Do N` (`self.NumFlashes`) :!label _label
    (:`Exit`
      (`SceneComponent.ToggleVisibility` (`self.PointLight`) false)
      (`KismetSystemLibrary.Delay` (`self.FlashInterval`))
      (`SceneComponent.ToggleVisibility` (`self.PointLight`) false)
      (`KismetSystemLibrary.Delay` (`self.FlashInterval`))
      (goto _label))))

(fn `NewFunction_0`
  (for _ (range 1)
    _))

(fn `UserConstructionScript`)